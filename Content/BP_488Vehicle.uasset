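; Player-driven race vehicle pawn that runs through a looping checkpoint sequence to win.
; Driving and camera input unlock once the game mode sets CanStart, after which Tick enforces a minimum forward throttle.
; Forward speed widens camera FOV on throttle input and drives the engine sound's RPM parameter.
; IncrementCheckpoints advances and reveals the next checkpoint, then CheckForWin triggers GameOver when the game mode's required count is reached.
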(event Custom|CheckForWin
  (bind _asagile_game_project_game_mode_base (Utilities|Casting|CastToAgileGameProjectGameModeBase (Game|GetGameMode)))
  (if (== (Variables|Default|GetCompletedCheckpoints) (Variables|/Script/AgileGameProject.AgileGameProjectGameModeBase|GetNumOfCheckpointsNeeded _asagile_game_project_game_mode_base))
    (for _array_element (Variables|Default|GetCheckpoint_array)
      (Rendering|SetActorHiddenInGame _array_element true)
      (Variables|/Script/Engine.PrimitiveComponent|SetbGenerateOverlapEvents (Variables|/Game/BP_Checkpoint.BP_Checkpoint_C|GetCube _array_element) false)
      (bind _output_get (Variables|/Script/AgileGameProject.AgileGameProjectGameModeBase|SetPlayerWin _asagile_game_project_game_mode_base true))
      (Class|AgileGameProjectGameModeBase|GameOver _asagile_game_project_game_mode_base _output_get))))

(event Custom|IncrementCheckpoints
  (params (Checkpoint :type BP%20Checkpoint%20Object%20Reference))
  (bind (_array_element _array_index) (Utilities|Array|ForEachLoopwithBreak (Variables|Default|GetCheckpoint_array) :!label _label)
    (:LoopBody
      (if (Utilities|Enum|Equal(Enum) (Utilities|GetDisplayName Checkpoint) (Utilities|GetDisplayName _array_element))
        (goto _label Break)))
    (:Completed
      (if (not (> (Variables|Default|GetCheckpointIndex) _array_index))
        (Rendering|SetActorHiddenInGame (Utilities|Array|Get(acopy) (Variables|Default|GetCheckpoint_array) (Variables|Default|GetCheckpointIndex)) true)
        (bind _result (Math|Integer|IncrementInt (Variables|Default|GetCheckpointIndex))
          (:%20%20
            (Variables|Default|SetCheckpointIndex _result)
            (bind _result_2 (Math|Integer|IncrementInt (Variables|Default|GetCompletedCheckpoints))
              (:%20%20
                (Variables|Default|SetCompletedCheckpoints _result_2)
                (if (> (Variables|Default|GetCheckpointIndex) (- (Utilities|Array|Length (Variables|Default|GetCheckpoint_array)) 1))
                  (bind _output_get (Variables|Default|SetCheckpointIndex 0))
                  (Rendering|SetActorHiddenInGame (Utilities|Array|Get(acopy) (Variables|Default|GetCheckpoint_array) _output_get) false)
                  (Variables|/Script/Engine.PrimitiveComponent|SetbGenerateOverlapEvents (Variables|/Game/BP_Checkpoint.BP_Checkpoint_C|GetCube (Utilities|Array|Get(acopy) (Variables|Default|GetCheckpoint_array) _output_get)) true)
                  (else
                    (Rendering|SetActorHiddenInGame (Utilities|Array|Get(acopy) (Variables|Default|GetCheckpoint_array) (Variables|Default|GetCheckpointIndex)) false)
                    (Variables|/Script/Engine.PrimitiveComponent|SetbGenerateOverlapEvents (Variables|/Game/BP_Checkpoint.BP_Checkpoint_C|GetCube (Utilities|Array|Get(acopy) (Variables|Default|GetCheckpoint_array) (Variables|Default|GetCheckpointIndex))) true)))
                (CallFunction|CheckforWin)))))))))

(event EventBeginPlay)

(event Collision|EventActorBeginOverlap
  (params (OtherActor :type Actor%20Object%20Reference)))

(event EventTick
  (params (DeltaSeconds :type Float%20%28single-precision%29))
  (Utilities|FlowControl|Sequence
    (:then_0
      (bind _asagile_game_project_game_mode_base (Utilities|Casting|CastToAgileGameProjectGameModeBase (Game|GetGameMode)))
      (if (Variables|/Script/AgileGameProject.AgileGameProjectGameModeBase|GetCanStart _asagile_game_project_game_mode_base)
        (if (Variables|Default|GetCanStart)
          (if (< (Variables|Default|GetThrottle) 0.1)
            (Class|WheeledVehicleMovementComponent|SetThrottleInput (Variables|Default|GetVehicleMovement) 0.1))
          (else
            (Variables|Default|SetCanStart (Variables|/Script/AgileGameProject.AgileGameProjectGameModeBase|GetCanStart _asagile_game_project_game_mode_base))))))
    (:then_1
      (Audio|Parameter|SetFloatParameter (Variables|Default|GetCarSound) "RPM" (Math|Float|Absolute(Float) (Class|WheeledVehicleMovementComponent|GetForwardSpeed (Variables|Default|GetVehicleMovement))) :!class /Script/Engine.AudioComponent))))

(event Input|ActionEvents|InputActionHandbrake
  (params (Key :type Key%20Structure :default "None"))
  (bind _canstart (Variables|Default|GetCanStart))
  (bind _vehiclemovement (Variables|Default|GetVehicleMovement))
  ;[1 1 1] Handbreak
  (:Pressed
    (if _canstart
      (Class|WheeledVehicleMovementComponent|SetHandbrakeInput _vehiclemovement true)))
  (:Released
    (if _canstart
      (Class|WheeledVehicleMovementComponent|SetHandbrakeInput _vehiclemovement false))))

(event Input|AxisEvents|InputAxisLookUp
  (params (AxisValue :type Float%20%28single-precision%29))
  ;[1 1 1] Camera Look Around
  (if (Variables|Default|GetCanStart)
    (Transformation|AddRelativeRotation (Variables|Default|GetSpringArm) (Math|Rotator|MakeRotator 0.0 AxisValue 0.0) false false)))

(event Input|AxisEvents|InputAxisLookRight
  (params (AxisValue :type Float%20%28single-precision%29))
  ;[1 1 1] Camera Look Around
  (if (Variables|Default|GetCanStart)
    (Transformation|AddRelativeRotation (Variables|Default|GetSpringArm) (Math|Rotator|MakeRotator 0.0 0.0 AxisValue) false false)))

(event Input|AxisEvents|InputAxisThrottle
  (params (AxisValue :type Float%20%28single-precision%29))
  (bind _carsound (Variables|Default|GetCarSound))
  (bind _vehiclemovement (Variables|Default|GetVehicleMovement))
  ;[1 1 1] Throttle and Steering
  (if (Variables|Default|GetCanStart)
    (bind _output_get (Variables|Default|SetThrottle AxisValue))
    (Class|WheeledVehicleMovementComponent|SetThrottleInput _vehiclemovement _output_get)
    (Camera|SetFieldOfView (Variables|Default|GetCamera) (+ (/ (Class|WheeledVehicleMovementComponent|GetForwardSpeed _vehiclemovement) 1e+02) 9e+01))
    (if (not (Audio|Components|Audio|IsPlaying _carsound))
      (Components|Activation|Activate _carsound false))))

(event Input|AxisEvents|InputAxisSteer
  (params (AxisValue :type Float%20%28single-precision%29))
  ;[1 1 1] Throttle and Steering
  (if (Variables|Default|GetCanStart)
    (Class|WheeledVehicleMovementComponent|SetSteeringInput (Variables|Default|GetVehicleMovement) AxisValue)))

(fn ConstructionScript)