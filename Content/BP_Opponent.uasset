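; BP_Opponent is an AI opponent vehicle that drives itself along a spline track at constant partial throttle.
; Each tick it gathers all Spline actors and passes them to GetPath, which follows the first one.
; GetPath projects a look-ahead point along the nearest tangent, farther at higher speed, then snaps it back onto the spline.
; The clamped yaw difference toward that point becomes the steering input.
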(event EventTick
  (params (DeltaSeconds :type Float%20%28single-precision%29))
  (bind _vehiclemovement (Variables|Default|GetVehicleMovement))
  (bind _outactors (Actor|GetAllActorsOfClass "/Game/Spline.Spline_C"))
  (bind _steering (CallFunction|GetPath _outactors))
  (Class|WheeledVehicleMovementComponent|SetSteeringInput _vehiclemovement _steering)
  (Class|WheeledVehicleMovementComponent|SetThrottleInput _vehiclemovement 0.75))

(fn ConstructionScript)

(fn GetPath
  (params (Spline :type Array%20of%20Spline%20Object%20References))
  (bind _returnvalue (Transformation|GetActorLocation))
  (bind _output (Utilities|Array|Get(acopy) Spline))
  (return (Math|Float|MapRangeClamped (.yaw (Math|Rotator|Delta(Rotator) (Math|Rotator|FindLookatRotation _returnvalue (Spline|FindLocationClosesttoWorldLocation (Variables|/Game/Spline.Spline_C|GetSpline _output) (+ (* (Math|Vector|Normalize (Class|SplineComponent|FindTangentClosesttoWorldLocation (Variables|/Game/Spline.Spline_C|GetSpline _output) _returnvalue "World")) (Math|Float|MapRangeClamped (CallFunction|GetCurrentSpeed) 2e+01 8e+01 5e+01 5e+02)) _returnvalue) "World")) (Transformation|GetActorRotation))) -9e+01 9e+01 -1.0 1.0)))

(fn GetCurrentSpeed
  (return (* (Class|WheeledVehicleMovementComponent|GetForwardSpeed (Variables|Default|GetVehicleMovement)) 0.36)) ; Return float Speed
)